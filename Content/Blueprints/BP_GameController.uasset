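; BP_GameController runs the overall game session, handling the HUD, music and win/lose ending.
; On BeginPlay it creates WBP_HUD, switches to game-and-UI input and plays the background soundtrack.
; EndGame(Win) fires once via a GameEnded flag, playing a victory or defeat sound.
; It then fades the HUD out and, after a short delay, shows WBP_EndGame with the result.
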(event `self.ReceiveBeginPlay`
  (bind _returnvalue (`GameplayStatics.GetPlayerController` 0))
  (`|ExecutionSequence`
    (:`then_0`
      ;[1 1 1] UI
      (bind _returnvalue_2 (`|CreateWidget` "/Game/Blueprints/UI/WBP_HUD.WBP_HUD_C" _returnvalue))
      (set `self.HUD` _returnvalue_2)
      (`UserWidget.AddToViewport` _returnvalue_2 0)
      (`WidgetBlueprintLibrary.SetInputMode_GameAndUIEx` _returnvalue _returnvalue_2 "DoNotLock" false)
      (`self.EnableInput` _returnvalue))
    (:`then_1`
      (`GameplayStatics.PlaySound2D` "/Game/Audio/Zombie_Survival_OST_HQ__Full_Soundtrack_.Zombie_Survival_OST_HQ__Full_Soundtrack_" 0.4 1.0 0.0 null null) ; play background music
    )))

(event `EndGame`
  (params (win :type Boolean))
  (if (`self.GameEnded`)
    (`KismetSystemLibrary.PrintString` "game already ended")
    (else
      (`|ExecutionSequence`
        (:`then_0`
          (set `self.GameEnded` true)
          ;[1 1 1] play victory/defeat sound
          (`GameplayStatics.PlaySound2D` (select `bool` win :`false` "/Game/Audio/creepy-girl-says-game-over-103538.creepy-girl-says-game-over-103538" :`true` "/Game/Audio/success-fanfare-trumpets-6185.success-fanfare-trumpets-6185" :!type "SoundBase Object Reference") (`KismetMathLibrary.SelectFloat` 1.0 4.0 win) 1.0 0.0 null null))
        (:`then_1`
          ;[1 1 1] set end game UI
          (`/Game/Blueprints/UI/WBP_HUD.PlayFadeOut` (`self.HUD`))
          (`KismetSystemLibrary.Delay` 1.0)
          (bind _returnvalue (`|CreateWidget` "/Game/Blueprints/UI/WBP_EndGame.WBP_EndGame_C" (`GameplayStatics.GetPlayerController` 0)))
          (`UserWidget.AddToViewport` _returnvalue 0)
          (`/Game/Blueprints/UI/WBP_EndGame.SetResult` _returnvalue win))))))

(fn `UserConstructionScript`)