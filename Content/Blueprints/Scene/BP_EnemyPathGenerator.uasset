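; Scene actor that builds a randomized, zigzag enemy path to the base at BeginPlay.
; Main points step along X from Max toward Min, alternating Y halves away from center, and end at the base.
; Corner points between them make right-angled segments.
; The points feed a spawned BP_EnemyPath, whose spline then drives the obstacle generator; a debug option builds a simplified path.
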(event `self.ReceiveBeginPlay`
  (bind _path (`self.path`))
  (bind _generatedpoints (`self.generatedPoints`))
  (bind _generatedpoints_2 (`self.generatedPoints`))
  (bind _output (`|GetArrayItem` _generatedpoints_2 (- (`KismetArrayLibrary.Array_Length` _generatedpoints_2) 1)))
  (set `self.halfStepSize` (/ (`self.StepSize`) 2.0))
  (bind _returnvalue (`|SpawnActorFromClass` "/Game/Blueprints/Scene/BP_EnemyPath.BP_EnemyPath_C" (`KismetMathLibrary.MakeTransform` (0.0 0.0 0.0) (struct) (1.0 1.0 0.2)) "Undefined" "OverrideRootScale" null null))
  (set `self.path` _returnvalue)
  (set `self.currentPos` (`self.Max`))
  (`SplineComponent.ClearSplinePoints` (`/Game/Blueprints/Scene/BP_EnemyPath.Spline` _returnvalue) true) ; this doesnt work..
  ;[1 1 1] generate main path points and connection point
  (bind _result (`self.GenerateMainPathPoints`))
  (for (_array_element _array_index) _result
    (`KismetArrayLibrary.Array_Add` (`self.generatedPoints`) _array_element)
    (if (< _array_index (- (`KismetArrayLibrary.Array_Length` _result) 1))
      (bind _connectpoint (`self.GenerateConnectPoint` _array_element (`|GetArrayItem` _result (+ _array_index 1))))
      (`KismetArrayLibrary.Array_Add` (`self.generatedPoints`) _connectpoint)))
  (if (`/Game/Blueprints/BP_Debug.SimplePath` (`self.Debug`))
    (`KismetArrayLibrary.Array_Set` _generatedpoints_2 0 (+ _output (* (`KismetMathLibrary.Normal` (- (`|GetArrayItem` _generatedpoints_2) _output)) (`self.debugFirstPathNodeDistance`)))))
  (for (_array_element_2 _array_index_2) _generatedpoints
    (if (`/Game/Blueprints/BP_Debug.SimplePath` (`self.Debug`))
      (if (or (<= _array_index_2 0) (> _array_index_2 (- (`KismetArrayLibrary.Array_Length` _generatedpoints) 3)))
        (`/Game/Blueprints/Scene/BP_EnemyPath.AddPoint` (`self.path`) _array_element_2 :!label _label))
      (else
        (goto _label))))
  (`/Game/Blueprints/Scene/BP_EnemyPath.Generate` _path)
  (`/Game/Blueprints/Scene/Obstackle/BP_ObstackleGenerator.Generate` (`self.ObstackleGenegator`) (`/Game/Blueprints/Scene/BP_EnemyPath.Spline` _path)))

(fn `GenerateConnectPoint`
  (params (Start :type "Vector Structure") (End :type "Vector Structure"))
  (returns (ConnectPoint :type "Vector Structure"))
  (return (`KismetMathLibrary.MakeVector` End_X Start_Y)))

(fn `GenerateMainPathPoints`
  (returns (result :type "Array of Vector Structure"))
  (locals (stepsCount :type Integer) (resultPoints :type "Array of Vector Structure") (CenterY :type "Float (double-precision)"))
  (bind (_max_x _max_y) (`KismetMathLibrary.BreakVector` (`self.Max`)))
  (bind (_min_x _min_y) (`KismetMathLibrary.BreakVector` (`self.Min`)))
  (bind (_max_x_2 _max_y_2) (`KismetMathLibrary.BreakVector` (`self.Max`)))
  (bind _resultpoints (`local.resultPoints`))
  (bind (_min_x_2 _min_y_2) (`KismetMathLibrary.BreakVector` (`self.Min`)))
  (bind _max_x_3 (`KismetMathLibrary.BreakVector` (`self.Max`)))
  (bind _centery (`local.CenterY`))
  (bind _minnodedistfromcenter (`self.MinNodeDistFromCenter`))
  (bind (_min_x_3 _min_y_3) (`KismetMathLibrary.BreakVector` (`self.Min`)))
  (bind (_max_x_4 _max_y_3) (`KismetMathLibrary.BreakVector` (`self.Max`)))
  (bind _resultpoints_2 (`local.resultPoints`))
  (set `local.CenterY` (/ (+ _max_y_3 _min_y_3) 2.0))
  (bind _output_get (set `local.stepsCount` (`KismetMathLibrary.FTrunc` (/ (- _max_x_4 _min_x_3) (`self.StepSize`)))))
  (for _index (range (+ _output_get 1))
    (if (> _index 0)
      (bind _returnvalue (- _max_x_3 (* _index (`self.StepSize`))))
      (bind (_output_x _output_y) (`KismetMathLibrary.BreakVector` (`|GetArrayItem` (`local.resultPoints`) (- _index 1))))
      (`KismetArrayLibrary.Array_Add` _resultpoints (`KismetMathLibrary.MakeVector` _returnvalue (`KismetMathLibrary.SelectFloat` (`KismetMathLibrary.RandomFloatInRange` _min_y (- _centery _minnodedistfromcenter)) (`KismetMathLibrary.RandomFloatInRange` (+ _centery _minnodedistfromcenter) _max_y) (> _output_y (`local.CenterY`)))))
      (else
        (`KismetArrayLibrary.Array_Add` _resultpoints (`KismetMathLibrary.MakeVector` _returnvalue (`KismetMathLibrary.RandomFloatInRange` _min_y_2 _max_y_2))))))
  (`KismetArrayLibrary.Array_Add` _resultpoints_2 (`self.K2_GetActorLocation` (`self.Base`)))
  (return _resultpoints_2))

(fn `UserConstructionScript`)