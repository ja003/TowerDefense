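; BP_EnemyPath is a spline-based enemy path actor that assigns itself to the BP_EnemySpawner on BeginPlay.
; Its construction script runs Generate, adding one collidable spline mesh per segment on a custom object channel.
; Tangents at interior points are flattened, with Y magnitude matched to X, so turns are orthogonal, while both endpoints keep standard tangents.
; AddPoint appends spline points using an incrementing input key, without regenerating meshes.
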(event `self.ReceiveBeginPlay`
  (bind _returnvalue (`GameplayStatics.GetActorOfClass` "/Game/Blueprints/BP_Debug.BP_Debug_C"))
  (set `self.debug` _returnvalue)
  (bind _returnvalue_2 (`GameplayStatics.GetActorOfClass` "/Game/Blueprints/Enemy/BP_EnemySpawner.BP_EnemySpawner_C"))
  (set `/Game/Blueprints/Enemy/BP_EnemySpawner.path` self _returnvalue_2))

(fn `AddPoint`
  (params (Point :type "Vector Structure"))
  (`SplineComponent.AddPoint` (`self.Spline`) (make `SplinePoint` (`self.inputKey`) Point) true)
  (set `self.inputKey` (+ (`self.inputKey`) 1.0)))

(fn `Generate`
  (locals (index :type Integer))
  (bind _spline (`self.Spline`))
  (bind _pathpointscale (`self.pathPointScale`))
  (for _index (range (+ (- (`SplineComponent.GetNumberOfSplinePoints` (`self.Spline`)) 2) 1))
    (bind _returnvalue (`AddComponent|NODE_AddSplineMeshComponent-0`))
    (`SplineMeshComponent.SetStartScale` _returnvalue _pathpointscale true)
    (`SplineMeshComponent.SetEndScale` _returnvalue _pathpointscale true)
    (`PrimitiveComponent.SetCollisionObjectType` _returnvalue "ECC_GameTraceChannel3")
    (`SplineMeshComponent.SetForwardAxis` _returnvalue "X" true)
    (`PrimitiveComponent.SetCollisionEnabled` _returnvalue "QueryAndPhysics")
    (set `local.index` _index)
    (bind _returnvalue_2 (`SplineComponent.GetTangentAtSplinePoint` _spline _index "Local"))
    (bind _returnvalue_3 (`KismetMathLibrary.SelectVector` _returnvalue_2 (`self.GetSameLengthVector` _returnvalue_2) (== (`local.index`) 0)))
    (bind _returnvalue_4 (+ _index 1))
    (bind _returnvalue_5 (`SplineComponent.GetTangentAtSplinePoint` _spline _returnvalue_4 "Local"))
    (bind _returnvalue_6 (`KismetMathLibrary.SelectVector` _returnvalue_5 (`self.GetSameLengthVector` _returnvalue_5) (== (`local.index`) (- (`SplineComponent.GetNumberOfSplinePoints` (`self.Spline`)) 2))))
    (`SplineMeshComponent.SetStartAndEnd` _returnvalue (`SplineComponent.GetLocationAtSplinePoint` _spline _index "Local") _returnvalue_3 (`SplineComponent.GetLocationAtSplinePoint` _spline _returnvalue_4 "Local") _returnvalue_6 true)
    (`KismetSystemLibrary.PrintText` (`|FormatText` "start = {s}, end = {e}" (`KismetStringLibrary.Conv_VectorToString` _returnvalue_3) (`KismetStringLibrary.Conv_VectorToString` _returnvalue_6)) :!enabledstate Disabled)))

(fn `GetSameLengthVector`
  (params (vector :type "Vector Structure"))
  (returns (result :type "Vector Structure"))
  (return (`KismetMathLibrary.MakeVector` vector_X (* (`KismetMathLibrary.Abs` vector_X) (`KismetMathLibrary.SignOfFloat` vector_Y)))))

(fn `UserConstructionScript`
  (`self.Generate`))