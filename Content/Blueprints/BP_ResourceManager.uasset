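; Resource manager Blueprint that tracks the player's coins in a tower defense game.
; On BeginPlay it loads starting coins and income from a data table, then runs a self-recalling one-second income loop.
; Tower purchases, half-price refunds and enemy rewards use enum-named data table rows and all change coins through AddCoins.
; A MegaCoins flag on BP_Debug grants bonus coins at startup.
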(event `self.ReceiveBeginPlay`
  (bind _returnvalue (`|GetDataTableRow` "/Game/Data/GameDataTable.GameDataTable" "game")
    (:`then`
      (set `self.coinsIncrement` (break `/Game/Data/GameData` _returnvalue))
      (set `self.Coins` (`.initCoins_16_D7AC3EA24CBBB4C25D6403B7DA162CD4` (break `/Game/Data/GameData` _returnvalue)))
      (`KismetSystemLibrary.Delay` 1.0)
      (`self.IncreaseCoins`)
      (bind _returnvalue_2 (`GameplayStatics.GetActorOfClass` "/Game/Blueprints/BP_Debug.BP_Debug_C"))
      (if (`/Game/Blueprints/BP_Debug.MegaCoins` _returnvalue_2)
        (`self.AddCoins` 999)))))

(event `IncreaseCoins`
  (`self.AddCoins` (`self.coinsIncrement`))
  (`KismetSystemLibrary.Delay` 1.0)
  (`self.IncreaseCoins`))

(fn `AddCoins`
  (params (increment :type Integer))
  (set `self.Coins` (+ (`self.Coins`) increment)))

(fn `CanBuyTower`
  (params (TowerType :type "/Game/Blueprints/Tower/ETower Enum" :default "NewEnumerator0"))
  (returns (result :type Boolean))
  (return (>= (`self.Coins`) (`self.Get Tower Price` TowerType))))

(fn `Get Tower Price`
  (params (tower :type "/Game/Blueprints/Tower/ETower Enum" :default "NewEnumerator0"))
  (returns (price :type Integer))
  (bind _returnvalue (`|GetDataTableRow` "/Game/Data/TowerDataTable.TowerDataTable" (`KismetStringLibrary.Conv_StringToName` (`|GetEnumeratorNameAsString` tower)))
    (:`then`
      (return (`.price_4_DEBCF83E40BE41C1347F1F94E98B6E29` (break `/Game/Data/TowerData` _returnvalue))))))

(fn `OnDestroyTower`
  (params (tower :type "/Game/Blueprints/Tower/ETower Enum" :default "NewEnumerator0"))
  (`self.AddCoins` (/ (`self.Get Tower Price` tower) 2)))

(fn `PayForTower`
  (params (tower :type "/Game/Blueprints/Tower/ETower Enum" :default "NewEnumerator0"))
  (`self.AddCoins` (* (`self.Get Tower Price` tower) -1)))

(fn `ReceiveRewardForEnemy`
  (params (type :type "/Game/Blueprints/Enemy/EEnemy Enum" :default "NewEnumerator0"))
  (bind _returnvalue (`|GetDataTableRow` "/Game/Data/EnemyDataTable.EnemyDataTable" (`KismetStringLibrary.Conv_StringToName` (`|GetEnumeratorNameAsString` type)))
    (:`then`
      (`self.AddCoins` (`.reward_15_5A75822B45C9FEDD12C87E9CBB4A4C52` (break `/Game/Data/EnemyData` _returnvalue))))))

(fn `UserConstructionScript`)