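; BP_ObstackleGenerator scatters random obstacle actors beside a given spline.
; GenerateSpawnLocations takes the midpoint of every other spline segment and shifts it by a random distance to a random side.
; The sideways vector, labelled orthogonal, swaps the segment direction's X and Y without negation, so it is not always perpendicular.
; Generate spawns a random class from Obstackles at each location with random yaw, printing debug strings.
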(fn `Generate`
  (params (spline :type "SplineComponent Object Reference"))
  (locals (spawnLocations :type "Array of Vector Structure") (newLoc :type "Vector Structure"))
  (bind _obstackles (`self.Obstackles`))
  (for _index (range (+ (- (`SplineComponent.GetNumberOfSplinePoints` spline) 2) 1))
    (if (== (mod _index 2) 0)
      (bind _returnvalue (`SplineComponent.GetLocationAtSplinePoint` spline _index "World"))
      (bind _returnvalue_2 (`SplineComponent.GetLocationAtSplinePoint` spline (+ _index 1) "World"))
      (bind (_returnvalue_x _returnvalue_y) (`KismetMathLibrary.BreakVector` (`KismetMathLibrary.Normal` (- _returnvalue_2 _returnvalue))))
      (bind _output_get (set `local.newLoc` (+ (/ (+ _returnvalue _returnvalue_2) 2) (* (* (`KismetMathLibrary.MakeVector` _returnvalue_y _returnvalue_x 0.0) (`KismetMathLibrary.RandomFloatInRange` (`self.minObstackleOffset`) (`self.maxObstackleOffset`))) (`KismetMathLibrary.SelectInt` -1 1 (`KismetMathLibrary.RandomBool`))))))
      (`KismetArrayLibrary.Array_Add` (`local.spawnLocations`) _output_get)))
  (for _array_element (`local.spawnLocations`)
    (`KismetSystemLibrary.PrintString` "spawn?")
    (bind _returnvalue_3 (`|SpawnActorFromClass` (`|GetArrayItem` _obstackles (`KismetMathLibrary.RandomIntegerInRange` 0 (- (`KismetArrayLibrary.Array_Length` _obstackles) 1))) (`KismetMathLibrary.MakeTransform` _array_element (`KismetMathLibrary.MakeRotator` 0.0 0.0 (`KismetMathLibrary.RandomFloatInRange` 0.0 360.0))) "AlwaysSpawn" "OverrideRootScale" null null))
    (`KismetSystemLibrary.PrintString` (`KismetSystemLibrary.GetDisplayName` _returnvalue_3))
    (`KismetSystemLibrary.PrintString` (`KismetStringLibrary.Conv_VectorToString` _array_element))))

(fn `UserConstructionScript`)