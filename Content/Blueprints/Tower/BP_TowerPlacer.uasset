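; BP_TowerPlacer handles mouse-driven tower placement in a tower defense game.
; StartPlacement spawns an inactive tower of the chosen type, which Tick moves to cursor hits on BP_Ground that pass a minimum-spacing sphere overlap, drawn for debugging.
; Left click places the tower and charges BP_ResourceManager, while right click destroys it.
; A bounds check against BP_EnemyPathGenerator's extents exists but is disconnected.
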(event `self.ReceiveBeginPlay`
  (bind _returnvalue (`GameplayStatics.GetPlayerController` 0))
  (`self.EnableInput` _returnvalue)
  (bind _asbp_td_player_controller (cast `/Game/Blueprints/BP_TD_PlayerController` _returnvalue))
  (add `/Game/Blueprints/BP_TD_PlayerController.OnLeftMouseBtnClicked` _asbp_td_player_controller (delegate `OnLeftMouseBtnClicked`))
  (bind _returnvalue_2 (`GameplayStatics.GetActorOfClass` "/Game/Blueprints/BP_ResourceManager.BP_ResourceManager_C"))
  (set `self.Resources` _returnvalue_2)
  (bind _returnvalue_3 (`GameplayStatics.GetActorOfClass` "/Game/Blueprints/Enemy/BP_EnemyPathGenerator.BP_EnemyPathGenerator_C"))
  (set `self.PathGenerator` _returnvalue_3))

(event `OnLeftMouseBtnClicked`
  (bind _spawningtower (`self.SpawningTower`))
  ;[1 1 1] Tower placement
  (`/Engine/EditorBlueprintResources/StandardMacros.IsValid` _spawningtower ; is any tower being spawned
    (:`Is Valid`
      (`/Game/Blueprints/Tower/BP_TowerBase.OnPlaced` _spawningtower)
      (`/Game/Blueprints/BP_ResourceManager.PayForTower` (`self.Resources`) (`/Game/Blueprints/Tower/BP_TowerBase.GetType` _spawningtower))
      (set `self.SpawningTower` null) ; set placed tower to null
    )))

(event `InputAction|RightMouseBtn`
  (params (Key :type "Key Structure"))
  (bind _spawningtower (`self.SpawningTower`))
  (:`Pressed`
    (`/Engine/EditorBlueprintResources/StandardMacros.IsValid` _spawningtower ; is any tower being spawned
      (:`Is Valid`
        (`self.K2_DestroyActor` _spawningtower)
        (set `self.SpawningTower` null) ; set placed tower to null
      ))))

(event `self.ReceiveTick`
  (params (DeltaSeconds :type "Float (single-precision)"))
  (bind _spawningtower (`self.SpawningTower`))
  (bind _hitresult (`PlayerController.GetHitResultUnderCursorForObjects` (`GameplayStatics.GetPlayerController` 0) (`self.GroundPathObjectType`) true))
  (`/Engine/EditorBlueprintResources/StandardMacros.IsValid` _spawningtower ; is any tower being spawned
    (:`Is Valid`
      (if (== (`GameplayStatics.GetObjectClass` (`.HitActor` (`GameplayStatics.BreakHitResult` _hitresult))) "/Game/Blueprints/BP_Ground.BP_Ground_C")
        (if (`self.CanPlaceTowerAt` (`.Location` (`GameplayStatics.BreakHitResult` _hitresult)))
          (`self.K2_SetActorLocation` _spawningtower (`.Location` (`GameplayStatics.BreakHitResult` _hitresult)) false false))))))

(fn `CanPlaceTowerAt`
  (params (Position :type "Vector Structure"))
  (returns (result :type Boolean))
  (locals (pos :type "Vector Structure"))
  (bind _mintowerdistance (`self.MinTowerDistance`))
  (bind (_outactors _returnvalue) (`KismetSystemLibrary.SphereOverlapActors` Position _mintowerdistance (`self.TowerObjectType`) "/Game/Blueprints/Tower/BP_TowerBase.BP_TowerBase_C" (`|MakeArray` (`self.SpawningTower`) :!type "Actor Object Reference")))
  (`KismetSystemLibrary.DrawDebugSphere` Position _mintowerdistance)
  (return (not _returnvalue)))

(fn `StartPlacement`
  (params (TowerType :type "/Game/Blueprints/Tower/ETower Enum" :default "NewEnumerator0"))
  (bind _returnvalue (`|SpawnActorFromClass` (select `/Game/Blueprints/Tower/ETower` TowerType :`NewEnumerator0` "/Game/Blueprints/Tower/BP_Tower1.BP_Tower1_C" :`NewEnumerator1` "/Game/Blueprints/Tower/BP_Tower2.BP_Tower2_C" :!type "Actor Class Reference") (`KismetMathLibrary.MakeTransform` (0.0 0.0 0.0)) "Undefined" "OverrideRootScale" null null))
  (bind _asbp_tower_base (cast `/Game/Blueprints/Tower/BP_TowerBase` _returnvalue))
  (bind _output_get (set `self.SpawningTower` _asbp_tower_base))
  (set `/Game/Blueprints/Tower/BP_TowerBase.IsActive` false _output_get)
  (`/Game/Blueprints/Tower/BP_TowerBase.OnStartPlacement` _asbp_tower_base))

(fn `UserConstructionScript`)