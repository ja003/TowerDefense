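; BP_Missile is a short-lived tower shot visual that stretches a cone between two points rather than moving as a projectile.
; Its Spawn function places the actor at the midpoint of Start and End and rotates it to face End.
; It then scales the thin Cone's Z axis by the distance between the points and sets a half-second lifespan.
; The event graph and construction script are empty.
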(fn `Spawn`
  (params (Start :type "Vector Structure") (End :type "Vector Structure"))
  (`self.K2_SetActorLocation` (/ (+ Start End) (2.0 2.0 2.0)))
  (`self.K2_SetActorRotation` (`KismetMathLibrary.FindLookAtRotation` Start End))
  (`SceneComponent.SetWorldScale3D` (`self.Cone`) (`KismetMathLibrary.MakeVector` 0.1 0.1 (/ (`KismetMathLibrary.Vector_Distance` End Start) 100.0)))
  (`self.SetLifeSpan` 0.5))

(fn `UserConstructionScript`)