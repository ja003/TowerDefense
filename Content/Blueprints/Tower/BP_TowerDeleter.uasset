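; BP_TowerDeleter handles removing a placed tower with a mouse click while its IsDeleting flag is set.
; It binds to the player controller's left-click event, traces under the cursor for tower objects and destroys the BP_TowerBase it hits.
; Before destroying it, it notifies BP_ResourceManager with the tower's type, then leaves delete mode.
; A right click cancels delete mode, and nothing in this graph turns it on.
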(event `self.ReceiveBeginPlay`
  (bind _asbp_td_player_controller (cast `/Game/Blueprints/BP_TD_PlayerController` (`GameplayStatics.GetPlayerController` 0)))
  (add `/Game/Blueprints/BP_TD_PlayerController.OnLeftMouseBtnClicked` _asbp_td_player_controller (delegate `OnLeftMouseBtnClicked`))
  (bind _returnvalue (`GameplayStatics.GetActorOfClass` "/Game/Blueprints/BP_ResourceManager.BP_ResourceManager_C"))
  (set `self.Resources` _returnvalue))

(event `InputAction|RightMouseBtn`
  (params (Key :type "Key Structure"))
  (:`Pressed`
    (set `self.IsDeleting` false)))

(event `OnLeftMouseBtnClicked`
  (bind _hitresult (`PlayerController.GetHitResultUnderCursorForObjects` (`GameplayStatics.GetPlayerController` 0) (`self.TowerObjectType`) true))
  (if (`self.IsDeleting`)
    (`/Engine/EditorBlueprintResources/StandardMacros.IsValid` (`.HitActor` (`GameplayStatics.BreakHitResult` _hitresult))
      (:`Is Valid`
        (bind _asbp_tower_base (cast `/Game/Blueprints/Tower/BP_TowerBase` (`.HitActor` (`GameplayStatics.BreakHitResult` _hitresult))))
        (`/Game/Blueprints/BP_ResourceManager.OnDestroyTower` (`self.Resources`) (`/Game/Blueprints/Tower/BP_TowerBase.GetType` _asbp_tower_base))
        (`/Game/Blueprints/Tower/BP_TowerBase.Destroy` _asbp_tower_base)
        (set `self.IsDeleting` false)))))

(fn `UserConstructionScript`)