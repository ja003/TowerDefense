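; BP_TowerDestroyer runs the tower demolition mode, letting the player destroy a tower by clicking it.
; SetIsDestroying toggles the mode and cancels any pending placement on the TowerPlacer when turning it on.
; It binds to BP_TD_PlayerController mouse events: right-click exits the mode, left-click traces under the cursor for tower objects.
; A hit BP_TowerBase gets DestroyTower called and the mode ends, so each activation removes one tower.
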(event `self.ReceiveBeginPlay`
  (bind _asbp_td_player_controller (cast `/Game/Blueprints/BP_TD_PlayerController` (`GameplayStatics.GetPlayerController` 0)))
  (add `/Game/Blueprints/BP_TD_PlayerController.OnRightMouseBtnClicked` _asbp_td_player_controller (delegate `OnRightMouseBtnClicked`))
  (add `/Game/Blueprints/BP_TD_PlayerController.OnLeftMouseBtnClicked` _asbp_td_player_controller (delegate `OnLeftMouseBtnClicked`))
  (set `self.Resources` null))

(event `OnRightMouseBtnClicked`
  ;[1 1 1] cancel destroy mode
  (`self.SetIsDestroying` false))

(event `OnLeftMouseBtnClicked`
  (bind _hitresult (`PlayerController.GetHitResultUnderCursorForObjects` (`GameplayStatics.GetPlayerController` 0) (`self.towerObjectType`) true))
  ;[1 1 1] Destroy tower
  (if (`self.IsDestroying`)
    (`/Engine/EditorBlueprintResources/StandardMacros.IsValid` (`.HitActor` (`GameplayStatics.BreakHitResult` _hitresult))
      (:`Is Valid`
        (bind _asbp_tower_base (cast `/Game/Blueprints/Tower/BP_TowerBase` (`.HitActor` (`GameplayStatics.BreakHitResult` _hitresult))))
        (`/Game/Blueprints/Tower/BP_TowerBase.DestroyTower` _asbp_tower_base true)
        (set `self.IsDestroying` false)))))

(fn `SetIsDestroying`
  (params (value :type Boolean))
  (set `self.IsDestroying` value)
  (if value
    (`/Game/Blueprints/Tower/BP_TowerPlacer.CancelTowerPlacement` (`self.TowerPlacer`))))

(fn `UserConstructionScript`)