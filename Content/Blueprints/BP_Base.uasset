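; BP_Base is the base that enemies attack; losing all its health ends the game as a loss and triggers an explosion.
; Max health and a looping timed self-repair come from GameDataTable.
; Damage and repair both feed AddHealth, which toggles tiered smoke and fire effects.
; It also assigns enemies attack spots with randomized navigable positions, falling back to the first when full, and supplies the nearer of two path targets.
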(event `self.ReceiveBeginPlay`
  (bind _returnvalue (`|GetDataTableRow` "/Game/Data/GameDataTable.GameDataTable" "game")
    (:`then`
      (set `self.MaxHealth` (`.baseHealth_8_294B63174161925717A7E7BFE97CA56D` (break `/Game/Data/GameData` _returnvalue)))
      (set `self.Health` (`self.MaxHealth`))
      (`self.Repair`))))

(event `Repair`
  (bind _returnvalue (`|GetDataTableRow` "/Game/Data/GameDataTable.GameDataTable" "game")
    (:`then`
      (`self.AddHealth` (`.repairHealthIncrement_22_AF29C48844048A4F0D61CA82A01CC192` (break `/Game/Data/GameData` _returnvalue)))
      (`KismetSystemLibrary.Delay` (`KismetMathLibrary.Conv_IntToDouble` (`.repairCooldown_23_0A9034804CFB1C7387F6CE98EF9674DA` (break `/Game/Data/GameData` _returnvalue))))
      (`self.Repair`))))

(fn `AddHealth`
  (params (healthIncrement :type Integer))
  (bind _health (`self.Health`))
  (bind _maxhealth (`self.MaxHealth`))
  (bind _p_smoke__destroylvl1_ (`self.P_Smoke (destroyLvl1)`))
  (bind _p_fire__destroylvl3_ (`self.P_Fire (destroyLvl3)`))
  (bind _p_smoke1__destroylvl2_ (`self.P_Smoke1 (destroyLvl2)`))
  (bind _returnvalue (/ _health (`KismetMathLibrary.Conv_IntToDouble` _maxhealth)))
  (bind _output_get (set `self.Health` (`KismetMathLibrary.Min` (+ _health healthIncrement) _maxhealth)))
  (if (<= _output_get 0)
    (bind _returnvalue_2 (`GameplayStatics.GetActorOfClass` "/Game/Blueprints/BP_GameController.BP_GameController_C"))
    (`/Game/Blueprints/BP_GameController.EndGame` _returnvalue_2 false)
    (`ActorComponent.Activate` (`self.P_Explosion`) false)
    (else
      (if (< _returnvalue 0.8)
        (`ActorComponent.Activate` _p_smoke__destroylvl1_ false)
        (else
          (`ActorComponent.Deactivate` _p_smoke__destroylvl1_)))
      (if (< _returnvalue 0.6)
        (`ActorComponent.Activate` _p_smoke1__destroylvl2_ false)
        (else
          (`ActorComponent.Deactivate` _p_smoke1__destroylvl2_)))
      (if (< _returnvalue 0.3)
        (`ActorComponent.Activate` _p_fire__destroylvl3_ false)
        (else
          (`ActorComponent.Deactivate` _p_fire__destroylvl3_))))))

(fn `Get Attack Spot`
  (params (enemy :type "/Game/Blueprints/Enemy/BP_EnemyBase Object Reference"))
  (returns (result :type "Vector Structure"))
  (for _array_element (`self.AttackSpots`)
    (bind (_value _returnvalue) (`BlueprintMapLibrary.Map_Find` (`self.AssignedAttackSpots`) _array_element))
    (if (or (== _value enemy) (or (not (`KismetSystemLibrary.IsValid` _value)) (not _returnvalue)))
      (`BlueprintMapLibrary.Map_Add` (`self.AssignedAttackSpots`) _array_element enemy)
      (`KismetSystemLibrary.PrintText` (`|FormatText` "assigning spot {x}" (`KismetStringLibrary.Conv_VectorToString` _array_element)) :!enabledstate Disabled)
      (bind _randomlocation (`NavigationSystemV1.K2_GetRandomLocationInNavigableRadius` (+ (`self.K2_GetActorLocation`) _array_element) 50.0 null null))
      (return _randomlocation)))
  (`KismetSystemLibrary.PrintString` "no more free spots" :!enabledstate Disabled)
  (return (+ (`self.K2_GetActorLocation`) (`|GetArrayItem` (`self.AttackSpots`)))))

(fn `GetEnemyPathTarget`
  (params (fromNode :type "Vector Structure"))
  (returns (attackSpotWorldPos :type "Vector Structure"))
  (bind _returnvalue (+ (`self.K2_GetActorLocation`) (`self.EnemyPathTarget2`)))
  (bind _returnvalue_2 (+ (`self.K2_GetActorLocation`) (`self.EnemyPathTarget1`)))
  (if (< (`KismetMathLibrary.Vector_Distance` fromNode _returnvalue) (`KismetMathLibrary.Vector_Distance` fromNode _returnvalue_2))
    (return _returnvalue)
    (else
      (return _returnvalue_2))))

(fn `GetHealthPercetage`
  (returns (NewParam :type "Float (double-precision)"))
  (return (/ (`KismetMathLibrary.Conv_IntToDouble` (`self.Health`)) (`self.MaxHealth`))))

(fn `ReceiveDamage`
  (params (Damage :type Integer))
  (`self.AddHealth` (* Damage -1)))

(fn `UserConstructionScript`)