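; BP_Debug is a debug actor that provides keyboard shortcuts for testing gameplay.
; It enables input for player controller 0 on BeginPlay, then handles hard-wired keys.
; B, E and M damage the first BP_Base found, damage the first BP_EnemyBase found, and call EndGame(false) on BP_GameController.
; Add and Subtract step a TimeDilation variable, apply it as global time dilation and print it, with no clamping.
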(event EventBeginPlay
  (Input|EnableInput (Game|GetPlayerController 0)))

(event Input|KeyboardEvents|DebugKeyB
  (params (Key :type Key%20Structure :default "None") (ActionValue :type Input%20Action%20Value%20Structure))
  (:Pressed
    (bind _returnvalue (Actor|GetActorOfClass "/Game/Blueprints/BP_Base.BP_Base_C"))
    (Default|ReceiveDamage _returnvalue 50)))

(event Input|KeyboardEvents|DebugKeyE
  (params (Key :type Key%20Structure :default "None") (ActionValue :type Input%20Action%20Value%20Structure))
  (:Pressed
    (bind _returnvalue (Actor|GetActorOfClass "/Game/Blueprints/Enemy/BP_EnemyBase.BP_EnemyBase_C"))
    (Default|ReceiveDamage _returnvalue 5)))

(event Input|KeyboardEvents|DebugKeyAdd
  (params (Key :type Key%20Structure :default "None") (ActionValue :type Input%20Action%20Value%20Structure))
  (bind _timedilation (Variables|Default|GetTimeDilation))
  (:Pressed
    (Math|Float|IncrementFloat _timedilation
      (:%20%20
        (Utilities|Time|SetGlobalTimeDilation _timedilation)
        (Development|PrintString (Utilities|String|ToString(Float) _timedilation))))))

(event Input|KeyboardEvents|DebugKeyM
  (params (Key :type Key%20Structure :default "None") (ActionValue :type Input%20Action%20Value%20Structure))
  (:Pressed
    (bind _returnvalue (Actor|GetActorOfClass "/Game/Blueprints/BP_GameController.BP_GameController_C"))
    (Default|EndGame _returnvalue false)))

(event Input|KeyboardEvents|Subtract
  (params (Key :type Key%20Structure :default "None"))
  (bind _timedilation (Variables|Default|GetTimeDilation))
  (:Pressed
    (Math|Float|DecrementFloat _timedilation
      (:%20%20
        (Utilities|Time|SetGlobalTimeDilation _timedilation)
        (Development|PrintString (Utilities|String|ToString(Float) _timedilation))))))

(fn ConstructionScript)