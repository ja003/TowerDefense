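; Enemy spawner that continuously spawns a random enemy type at a random spawnpoint, starting shortly after BeginPlay.
; SpawnEnemy re-calls itself after a short delay to loop indefinitely, printing each spawned class name.
; SelectEnemyToSpawn maps a random EEnemy value to the simple or big enemy class.
; GetSpawnpoint picks a random Spawnpoints transform, but its Length minus one bound to RandomInteger excludes the last entry.
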(event `self.ReceiveBeginPlay`
  (`KismetSystemLibrary.Delay` 0.5)
  (`self.SpawnEnemy`))

(event `SpawnEnemy`
  (bind _enemytospawn (`self.EnemyToSpawn`))
  (`self.SelectEnemyToSpawn`)
  (bind _output (`self.GetSpawnpoint`))
  (`|SpawnActorFromClass` _enemytospawn _output "Undefined" "OverrideRootScale" null null)
  (`KismetSystemLibrary.PrintString` (`KismetSystemLibrary.GetClassDisplayName` _enemytospawn))
  (`KismetSystemLibrary.Delay` 1.0)
  (`self.SpawnEnemy`))

(fn `GetSpawnpoint`
  (returns (Output :type "Transform Structure (by ref)"))
  (bind _spawnpoints (`self.Spawnpoints`))
  (return (`|GetArrayItem` _spawnpoints (`KismetMathLibrary.RandomInteger` (- (`KismetArrayLibrary.Array_Length` _spawnpoints) 1)))))

(fn `SelectEnemyToSpawn`
  (set `self.EnemyTypeToSpawn` (cast `/Game/Blueprints/EEnemy` (`KismetMathLibrary.Conv_IntToByte` (`KismetMathLibrary.RandomInteger` (enumcount `/Game/Blueprints/EEnemy`)))))
  (switch `/Game/Blueprints/EEnemy` (`self.EnemyTypeToSpawn`)
    (:`NewEnumerator0`
      (set `self.EnemyToSpawn` "/Game/Blueprints/BP_EnemySimple.BP_EnemySimple_C"))
    (:`NewEnumerator1`
      (set `self.EnemyToSpawn` "/Game/Blueprints/BP_EnemyBig.BP_EnemyBig_C"))))

(fn `UserConstructionScript`)