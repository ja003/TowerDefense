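; BP_EnemyPathGenerator builds a randomized enemy path from Start toward End when play begins.
; It spawns a BP_EnemyPath and clears its spline, then repeatedly steps toward End, adding random XY jitter of up to half a step.
; Each point is appended and debug-printed until one lands within a step of End, which updates the spline before Generate is called.
; Start and End themselves are never added as points.
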(event `self.ReceiveBeginPlay`
  (bind _halfstepsize (`self.halfStepSize`))
  (bind _halfstepsize_2 (`self.halfStepSize`))
  (bind _returnvalue (- (`self.End`) (`self.currentPos`)))
  (set `self.halfStepSize` (/ (`self.stepSize`) 2.0))
  (bind _returnvalue_2 (`|SpawnActorFromClass` "/Game/Blueprints/Enemy/BP_EnemyPath.BP_EnemyPath_C" (`KismetMathLibrary.MakeTransform` (0.0 0.0 0.0) (struct) (1.0 1.0 0.2)) "Undefined" "OverrideRootScale" null null))
  (set `self.currentPos` (`self.Start`))
  (bind _spline (`/Game/Blueprints/Enemy/BP_EnemyPath.Spline` _returnvalue_2))
  (`SplineComponent.ClearSplinePoints` _spline false)
  (while (!= (`self.bEndReached`) true)
    (bind _output_get (set `self.currentPos` (+ (+ (`self.currentPos`) (* (`KismetMathLibrary.Normal` _returnvalue) (`self.stepSize`))) (`KismetMathLibrary.MakeVector` (`KismetMathLibrary.RandomFloatInRange` (* _halfstepsize_2 -1.0) _halfstepsize_2) (`KismetMathLibrary.RandomFloatInRange` (* _halfstepsize -1.0) _halfstepsize)))))
    (bind _output_get_2 (set `self.bEndReached` (< (`KismetMathLibrary.VSize` _returnvalue) (`self.stepSize`))))
    (`SplineComponent.AddPoint` _spline (make `SplinePoint` (`self.Input Key`) _output_get) _output_get_2)
    (`KismetSystemLibrary.PrintText` (`KismetTextLibrary.Conv_VectorToText` _output_get))
    (set `self.Input Key` (+ (`self.Input Key`) 1.0)))
  (`/Game/Blueprints/Enemy/BP_EnemyPath.Generate` _returnvalue_2))

(fn `UserConstructionScript`)