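; Enemy path actor that draws a spline as a chain of mesh segments and hands itself to the enemy spawner on BeginPlay.
; The construction script runs Generate, adding a scaled, collidable spline mesh between each point pair and printing its tangents.
; Interior tangents are flattened and forced diagonal by matching Y magnitude to X, while both path ends keep their original tangents.
; AddPoint appends spline points with an incrementing input key, without rebuilding meshes.
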(event `self.ReceiveBeginPlay`
  (bind _returnvalue (`GameplayStatics.GetActorOfClass` "/Game/Blueprints/BP_Debug.BP_Debug_C"))
  (set `self.Debug` _returnvalue)
  (bind _returnvalue_2 (`GameplayStatics.GetActorOfClass` "/Game/Blueprints/Enemy/BP_EnemySpawner.BP_EnemySpawner_C"))
  (set `/Game/Blueprints/Enemy/BP_EnemySpawner.Path` self _returnvalue_2))

(fn `AddPoint`
  (params (Point :type "Vector Structure"))
  (`SplineComponent.AddPoint` (`self.Spline`) (make `SplinePoint` (`self.InputKey`) Point) true)
  (set `self.InputKey` (+ (`self.InputKey`) 1.0)))

(fn `Generate`
  (locals (isFirst :type Boolean) (isLast :type Boolean))
  (bind _spline (`self.Spline`))
  (bind _pathpointscale (`self.PathPointScale`))
  (bind _returnvalue (- (`SplineComponent.GetNumberOfSplinePoints` (`self.Spline`)) 2))
  (for _index (range (+ _returnvalue 1))
    (set `local.isFirst` (== _index 0))
    (set `local.isLast` (== _index _returnvalue))
    (bind _returnvalue_2 (`AddComponent|NODE_AddSplineMeshComponent-0`))
    (`SplineMeshComponent.SetStartScale` _returnvalue_2 _pathpointscale true)
    (`SplineMeshComponent.SetEndScale` _returnvalue_2 _pathpointscale true)
    (`PrimitiveComponent.SetCollisionObjectType` _returnvalue_2 "ECC_GameTraceChannel3")
    (`SplineMeshComponent.SetForwardAxis` _returnvalue_2 "X" true)
    (`PrimitiveComponent.SetCollisionEnabled` _returnvalue_2 "QueryAndPhysics")
    (bind _returnvalue_3 (`SplineComponent.GetTangentAtSplinePoint` _spline _index "Local"))
    (bind _returnvalue_4 (`KismetMathLibrary.SelectVector` _returnvalue_3 (`self.GetSameLengthVector` _returnvalue_3) (`local.isFirst`)))
    (bind _returnvalue_5 (+ _index 1))
    (bind _returnvalue_6 (`SplineComponent.GetTangentAtSplinePoint` _spline _returnvalue_5 "Local"))
    (bind _returnvalue_7 (`KismetMathLibrary.SelectVector` _returnvalue_6 (`self.GetSameLengthVector` _returnvalue_6) (`local.isLast`)))
    (`SplineMeshComponent.SetStartAndEnd` _returnvalue_2 (`SplineComponent.GetLocationAtSplinePoint` _spline _index "Local") _returnvalue_4 (`SplineComponent.GetLocationAtSplinePoint` _spline _returnvalue_5 "Local") _returnvalue_7 true)
    (`KismetSystemLibrary.PrintText` (`|FormatText` "start = {s}, end = {e}" (`KismetStringLibrary.Conv_VectorToString` _returnvalue_4) (`KismetStringLibrary.Conv_VectorToString` _returnvalue_7)))))

(fn `GetSameLengthVector`
  (params (vector :type "Vector Structure"))
  (returns (result :type "Vector Structure"))
  (return (`KismetMathLibrary.MakeVector` vector_X (* (`KismetMathLibrary.Abs` vector_X) (`KismetMathLibrary.SignOfFloat` vector_Y)))))

(fn `UserConstructionScript`
  (`self.Generate`))