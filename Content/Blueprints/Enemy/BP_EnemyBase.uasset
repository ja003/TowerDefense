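; Base enemy character for a wave game, following a spline path to attack BP_Base.
; Init finds base and path, loads wave-scaled stats from EnemyDataTable by enemy type, and spawns a healthbar.
; Path nodes are offset perpendicular to the spline tangent by spawn index to spread enemies.
; TryAttack flags cooldown-gated attacks, DealDamage deals a fixed 1 ignoring the Damage stat, and Die notifies the spawner, leaving destruction to OnDeadAnimFinish.
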(event `self.ReceiveBeginPlay`
  (`self.SpawnDefaultController`))

(fn `DealDamage`
  (`/Game/Blueprints/BP_Base.ReceiveDamage` (`self.Base`) 1))

(fn `Die`
  (bind _returnvalue (`GameplayStatics.GetActorOfClass` "/Game/Blueprints/Enemy/BP_EnemySpawner.BP_EnemySpawner_C"))
  (`/Game/Blueprints/Enemy/BP_EnemySpawner.OnEnemyDeath` _returnvalue self)
  (set `self.IsDead` true)
  (`GameplayStatics.PlaySoundAtLocation` "/Game/Audio/Lego_Yoda_Death_-_Sound_Effect__HD_.Lego_Yoda_Death_-_Sound_Effect__HD_" (`self.K2_GetActorLocation`) (struct) 0.3 1.0 1.1 null null null null))

(fn `GetCurrentPathNode`
  (returns (node :type "Vector Structure"))
  (return (`SplineComponent.GetLocationAtSplinePoint` (`/Game/Blueprints/Enemy/BP_EnemyPath.Spline` (`self.Path`)) (`self.CurrentPathNodeIndex`) "Local")))

(fn `GetPathNode`
  (params (index :type Integer))
  (returns (node :type "Vector Structure"))
  (bind _spline (`/Game/Blueprints/Enemy/BP_EnemyPath.Spline` (`self.Path`)))
  (bind (_returnvalue_x _returnvalue_y) (`KismetMathLibrary.BreakVector` (`KismetMathLibrary.Normal` (`SplineComponent.GetTangentAtSplinePoint` _spline index "Local"))))
  (return (+ (`SplineComponent.GetLocationAtSplinePoint` _spline index "Local") (* (`KismetMathLibrary.MakeVector` (* _returnvalue_y -1.0) _returnvalue_x) (`self.GetPathOffset`)))))

(fn `GetPathOffset`
  (returns (offset :type "Float (double-precision)"))
  (locals (spawnOffsetmultiply :type "Map of Integer to Float (double-precision)") (spawnOffsetMax :type Integer :default 50))
  (bind _spawnoffsetmultiply (`local.spawnOffsetmultiply`))
  (return (* (`local.spawnOffsetMax`) (`BlueprintMapLibrary.Map_Find` _spawnoffsetmultiply (mod (`self.SpawnIndex`) (`BlueprintMapLibrary.Map_Length` _spawnoffsetmultiply))))))

(fn `GetType`
  (returns (type :type "/Game/Blueprints/Enemy/EEnemy Enum"))
  (return "NewEnumerator0"))

(fn `Init`
  (params (wave :type Integer))
  (locals (waveIndex :type Integer))
  (set `local.waveIndex` wave)
  (bind _returnvalue (`GameplayStatics.GetActorOfClass` "/Game/Blueprints/BP_Base.BP_Base_C"))
  (set `self.Base` _returnvalue)
  (bind _returnvalue_2 (`GameplayStatics.GetActorOfClass` "/Game/Blueprints/Enemy/BP_EnemyPath.BP_EnemyPath_C"))
  (set `self.Path` _returnvalue_2)
  (bind _returnvalue_3 (`|GetDataTableRow` "/Game/Data/EnemyDataTable.EnemyDataTable" (`KismetStringLibrary.Conv_StringToName` (`|GetEnumeratorNameAsString` (`self.GetType`))))
    (:`then`
      (set `CharacterMovementComponent.MaxWalkSpeed` (+ (* (`local.waveIndex`) (`.speedIncrement_25_03CB02C2439F3FC4630B88BEFA884ED0` (break `/Game/Data/EnemyData` _returnvalue_3))) (`.speed_8_16995C474C819DAB285FACA00B220B63` (break `/Game/Data/EnemyData` _returnvalue_3))) (`self.CharacterMovement`))
      (bind _output_get (set `self.Health` (+ (* (`local.waveIndex`) (`.healthIncrement_18_927305A24CA3391F258375B33743DEBD` (break `/Game/Data/EnemyData` _returnvalue_3))) (break `/Game/Data/EnemyData` _returnvalue_3))))
      (set `self.MaxHealth` _output_get)
      (set `self.Damage` (+ (* (`local.waveIndex`) (`.damageIncrement_22_BBA0547F47EEE89DFE69E5BD86632873` (break `/Game/Data/EnemyData` _returnvalue_3))) (`.damage_7_890C26D54C6E56B9670AED876E9F1D63` (break `/Game/Data/EnemyData` _returnvalue_3))))
      (set `self.cooldown` (`.cooldown_12_7278268A45A85C5798CC5FBA027956C2` (break `/Game/Data/EnemyData` _returnvalue_3)))
      (bind _returnvalue_4 (`|SpawnActorFromClass` "/Game/Blueprints/BP_Healthbar.BP_Healthbar_C" (`KismetMathLibrary.MakeTransform` (`SceneComponent.RelativeLocation` (`self.HealthbarLocation`))) "Undefined" "OverrideRootScale" null null))
      (`self.SetNavModifierState` false)
      (bind _output_get_2 (set `self.healthbar` _returnvalue_4))
      (`self.K2_AttachToActor` _output_get_2 self "None" "KeepRelative" "KeepRelative" "KeepRelative" true))
    (:`RowNotFound`
      (`KismetSystemLibrary.PrintString` "error - data not found"))))

(fn `IsCloseToBase`
  (returns (result :type Boolean))
  (bind _returnvalue (`KismetMathLibrary.Vector_Distance2D` (`self.K2_GetActorLocation` (`self.Base`)) (`self.K2_GetActorLocation` self)))
  (`KismetSystemLibrary.PrintString` (`KismetStringLibrary.Conv_DoubleToString` _returnvalue) :!enabledstate Disabled)
  (return (< _returnvalue (`self.range`))))

(fn `IsInAttackRange`
  (returns (ReturnValue :type Boolean))
  (return (< (`KismetMathLibrary.Vector_Distance2D` (`self.K2_GetActorLocation` (`self.Base`)) (`self.K2_GetActorLocation`)) (`self.range`))))

(fn `OnDeadAnimFinish`
  (`self.K2_DestroyActor` (`self.healthbar`))
  (`self.K2_DestroyActor`))

(fn `ReceiveDamage`
  (params (Damage :type Integer))
  (returns (IsDead :type Boolean))
  (bind _output_get (set `self.Health` (- (`self.Health`) Damage)))
  (`/Game/Blueprints/BP_Healthbar.SetPercentage` (`self.healthbar`) (/ (`KismetMathLibrary.Conv_DoubleToFloat` (`KismetMathLibrary.Conv_IntToDouble` (`self.Health`))) (`self.MaxHealth`)))
  (bind _returnvalue (<= _output_get 0))
  (if _returnvalue
    (`self.Die`))
  (return _returnvalue))

(fn `SetNavModifierState`
  (params (active :type Boolean))
  (`NavModifierComponent.SetAreaClass` (`self.NavModifier`) (select `bool` active :`true` "/Script/NavigationSystem.NavArea_Null" :!type "NavArea Class Reference")))

(fn `TryAttack`
  (if (`self.IsInAttackRange`)
    (if (> (- (`GameplayStatics.GetTimeSeconds`) (`self.lastAttackTime`)) (`self.cooldown`))
      (set `self.lastAttackTime` (`GameplayStatics.GetTimeSeconds`))
      (set `self.IsAttacking` true))))

(fn `UserConstructionScript`)