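; Enemy spawner that runs waves of randomly picked Simple or Big enemies, sized per wave from the game data table.
; Each wave builds random type and delay arrays, then a self-calling event spawns enemies near the spline path's first point until done or game over.
; Emptying the active enemy list on death awards wave coins and starts the next wave; exhausting waves ends the game.
; Debug settings can force one enemy type or shrink waves.
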(event `self.ReceiveBeginPlay`
  (bind _returnvalue (`|GetDataTableRow` "/Game/Data/GameDataTable.GameDataTable" "game")
    (:`then`
      (bind _output_get (set `self.EnemyCountAtWave` (`.EnemyCountAtWave_13_334BF25B4F942D4F3590EC8208DD6595` (break `/Game/Data/GameData` _returnvalue))))
      (`KismetSystemLibrary.Delay` 0.2)
      (`self.GenerateNextWave` 0.0))))

(event `GenerateNextWave`
  (params (delay :type "Float (double-precision)"))
  (`KismetSystemLibrary.Delay` delay)
  (if (< (`self.CurrentWave`) (`BlueprintMapLibrary.Map_Length` (`self.EnemyCountAtWave`)))
    (`KismetSystemLibrary.PrintString` "next wave" :!enabledstate Disabled)
    (`/Engine/EditorBlueprintResources/StandardMacros.IncrementInt` (`self.CurrentWave`)
      (:`  `
        (bind (_enemies _spawndelay) (`self.GetWave`))
        (`self.TryGenerateEnemy` _enemies _spawndelay)))
    (else
      (bind _returnvalue (`GameplayStatics.GetActorOfClass` "/Game/Blueprints/BP_GameController.BP_GameController_C"))
      (`/Game/Blueprints/BP_GameController.EndGame` _returnvalue true))))

(event `TryGenerateEnemy`
  (params (enemies :type "Array of /Game/Blueprints/Enemy/EEnemy Enum") (spawnDelays :type "Array of Float (double-precision)") (index :type Integer))
  (if (`/Game/Blueprints/BP_GameController.GameEnded` (`self.Game`))
    (`KismetSystemLibrary.PrintString` "game over - stop spawn")
    (elif (< index (`KismetArrayLibrary.Array_Length` enemies))
      (`KismetSystemLibrary.PrintString` "try gen next" :!enabledstate Disabled)
      (`KismetSystemLibrary.Delay` (`|GetArrayItem` spawnDelays index))
      (bind _spawnedactor (`self.SpawnEnemy` (`|GetArrayItem` enemies index)))
      (`BlueprintSetLibrary.Set_Add` (`self.ActiveEnemies`) _spawnedactor)
      (bind _result (`/Engine/EditorBlueprintResources/StandardMacros.IncrementInt` index)
        (:`  `
          (`self.TryGenerateEnemy` enemies spawnDelays _result)))
      (else
        (`KismetSystemLibrary.PrintString` "no more enemies" :!enabledstate Disabled)))))

(fn `GetEnemyActor`
  (params (enemyType :type "/Game/Blueprints/Enemy/EEnemy Enum" :default "NewEnumerator0"))
  (returns (enemy :type "/Game/Blueprints/Enemy/BP_EnemyBase Class Reference"))
  (bind _spawnenemy (`/Game/Blueprints/BP_Debug.SpawnEnemy` (`self.Debug`)))
  (switch `/Game/Blueprints/Enemy/EEnemy` _spawnenemy
    (:`NewEnumerator2`
      (return (select `/Game/Blueprints/Enemy/EEnemy` enemyType :`NewEnumerator0` "/Game/Blueprints/Enemy/BP_EnemySimple.BP_EnemySimple_C" :`NewEnumerator1` "/Game/Blueprints/Enemy/BP_EnemyBig.BP_EnemyBig_C" :!type "/Game/Blueprints/Enemy/BP_EnemyBase Class Reference")))
    (:`NewEnumerator0`
      _)
    (:`NewEnumerator1`
      _))
  (return (select `/Game/Blueprints/Enemy/EEnemy` _spawnenemy :`NewEnumerator0` "/Game/Blueprints/Enemy/BP_EnemySimple.BP_EnemySimple_C" :`NewEnumerator1` "/Game/Blueprints/Enemy/BP_EnemyBig.BP_EnemyBig_C" :!type "/Game/Blueprints/Enemy/BP_EnemyBase Class Reference")))

(fn `GetSpawnpoint`
  (returns (Output :type "Transform Structure (by ref)"))
  (locals (spawnOffset :type "Float (double-precision)" :default 50.0))
  (bind _spawnoffset (`local.spawnOffset`))
  (bind _returnvalue (* _spawnoffset -1.0))
  (return (`KismetMathLibrary.Conv_VectorToTransform` (+ (`SplineComponent.GetLocationAtSplinePoint` (`/Game/Blueprints/Enemy/BP_EnemyPath.Spline` (`self.Path`)) 0 "Local") (`KismetMathLibrary.MakeVector` (`KismetMathLibrary.RandomFloatInRange` _returnvalue _spawnoffset) (`KismetMathLibrary.RandomFloatInRange` _returnvalue _spawnoffset) 100.0)))))

(fn `GetWave`
  (returns (enemies :type "Array of /Game/Blueprints/Enemy/EEnemy Enum") (spawnDelay :type "Array of Float (double-precision)"))
  (locals (resultEnemies :type "Array of /Game/Blueprints/Enemy/EEnemy Enum") (resultSpawnDelays :type "Array of Float (double-precision)"))
  (for _ (range (+ (`KismetMathLibrary.SelectInt` 0 (`BlueprintMapLibrary.Map_Find` (`self.EnemyCountAtWave`) (`self.CurrentWave`)) (`/Game/Blueprints/BP_Debug.OneEnemy` (`self.Debug`))) 1))
    (`KismetArrayLibrary.Array_Add` (`local.resultEnemies`) (cast `/Game/Blueprints/Enemy/EEnemy` (`KismetMathLibrary.Conv_IntToByte` (`KismetMathLibrary.RandomIntegerInRange` 1 (- (enumcount `/Game/Blueprints/Enemy/EEnemy`) 1)))))
    (`KismetArrayLibrary.Array_Add` (`local.resultSpawnDelays`) (`KismetMathLibrary.RandomFloatInRange` 1.5 4.0)))
  (return (`local.resultEnemies`) (`local.resultSpawnDelays`)))

(fn `OnEnemyDeath`
  (params (enemy :type "/Game/Blueprints/Enemy/BP_EnemyBase Object Reference"))
  (bind _activeenemies (`self.ActiveEnemies`))
  (bind _returnvalue (`BlueprintSetLibrary.Set_Length` _activeenemies))
  (`BlueprintSetLibrary.Set_Remove` _activeenemies enemy)
  (`KismetSystemLibrary.PrintText` (`|FormatText` "{x} / {y} enemies left" _returnvalue (`BlueprintMapLibrary.Map_Find` (`self.EnemyCountAtWave`) (`self.CurrentWave`))))
  (if (== _returnvalue 0)
    (`KismetSystemLibrary.PrintString` "last enemy killed - another wave")
    (bind _returnvalue_2 (`|GetDataTableRow` "/Game/Data/GameDataTable.GameDataTable" "game")
      (:`then`
        (`/Game/Blueprints/BP_ResourceManager.AddCoins` (`self.Resources`) (`BlueprintMapLibrary.Map_Find` (`.EnemyRewardAtWave_28_6CBB00F44034F7B9C5C144A17D2A05F6` (break `/Game/Data/GameData` _returnvalue_2)) (`self.CurrentWave`)))
        (`self.GenerateNextWave` 3.0)))))

(fn `SpawnEnemy`
  (params (enemy :type "/Game/Blueprints/Enemy/EEnemy Enum" :default "NewEnumerator0"))
  (returns (spawnedActor :type "/Game/Blueprints/Enemy/BP_EnemyBase Object Reference"))
  (bind _output (`self.GetSpawnpoint`))
  (bind _enemyspawnindex (`self.EnemySpawnIndex`))
  (bind _returnvalue (`|SpawnActorFromClass` (`self.GetEnemyActor` enemy) _output "AdjustIfPossibleButAlwaysSpawn" "OverrideRootScale" null null))
  (`GameplayStatics.PlaySoundAtLocation` "/Game/Audio/zombie-spawn.zombie-spawn" (`KismetMathLibrary.TransformLocation` _output) (struct) 0.4 1.0 0.0 null null null null)
  (`/Engine/EditorBlueprintResources/StandardMacros.IsValid` _returnvalue
    (:`Is Valid`
      (`/Game/Blueprints/Enemy/BP_EnemyBase.Init` _returnvalue (`self.CurrentWave`))
      (set `/Game/Blueprints/Enemy/BP_EnemyBase.SpawnIndex` _enemyspawnindex _returnvalue)
      (`/Engine/EditorBlueprintResources/StandardMacros.IncrementInt` _enemyspawnindex
        (:`  `
          (return _returnvalue))))
    (:`Is Not Valid`
      (`KismetSystemLibrary.PrintString` "error: enemy not spawned"))))

(fn `UserConstructionScript`)